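; BP_Malty is a playable character with camera-look, movement and interaction through Enhanced Input, playing an idle hand montage on start.
; Movement input runs at half scale unless the dash input is held, while XSpeed and YSpeed record strafe input and horizontal speed.
; A camera line trace each tick writes the targeted actor's display name to WBP_PlayerUI.
; Interact repeats the trace and sends the hit actor an interface message.
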(event `self.ReceiveBeginPlay`
  (set `self.XSpeed` 0.0)
  (set `self.YSpeed` 0.0)
  (bind _foundwidgets (`WidgetBlueprintLibrary.GetAllWidgetsOfClass` "/Game/Blueprint/GUI/WBP_PlayerUI.WBP_PlayerUI_C"))
  (set `self.Player_UI` (`|GetArrayItem` _foundwidgets))
  (`|PlayMontage` (`self.Mesh`) "/Game/3D_Model/Player_Malty/Anim/AM_Malty_Hand.AM_Malty_Hand" 1.0 0.0 "Idle"))

(event `self.ReceiveTick`
  (params (DeltaSeconds :type "Float (single-precision)"))
  (set `self.YSpeed` (`KismetMathLibrary.VSizeXY` (`self.GetVelocity`)))
  (bind _outhit (`KismetSystemLibrary.LineTraceSingle` (`SceneComponent.K2_GetComponentLocation` (`self.Camera`)) (`SceneComponent.K2_GetComponentLocation` (`self.Line_Direction`)) "TraceTypeQuery1"))
  (bind (_bblockinghit _binitialoverlap _time _distance _location _impactpoint _normal _impactnormal _physmat _hitactor) (`GameplayStatics.BreakHitResult` _outhit))
  (`/Engine/EditorBlueprintResources/StandardMacros.IsValid` _hitactor
    (:`Is Valid`
      (bind _display_name (message `/Game/Blueprint/BPI_Interactable.GetDisplayName` _hitactor))
      (set `/Game/Blueprint/GUI/WBP_PlayerUI.Current_Object_Name` _display_name (`self.Player_UI`)))
    (:`Is Not Valid`
      (set `/Game/Blueprint/GUI/WBP_PlayerUI.Current_Object_Name` "" (`self.Player_UI`)))))

(event `EnhancedInput|/Game/Blueprint/Input/IA_Movement`
  (params (ActionValue :type "Vector2D Structure") (ElapsedSeconds :type "Float (double-precision)") (TriggeredSeconds :type "Float (double-precision)") (InputAction :type "InputAction Object Reference" :default "/Game/Blueprint/Input/IA_Movement.IA_Movement"))
  (bind _returnvalue (`self.K2_GetActorRotation`))
  (bind _returnvalue_2 (`KismetMathLibrary.GetForwardVector` _returnvalue))
  (bind _returnvalue_3 (`KismetMathLibrary.GetRightVector` _returnvalue))
  (:`Triggered`
    (set `self.XSpeed` ActionValue_X :!label _label)
    (if (`self.IsDash`)
      (`self.AddMovementInput` _returnvalue_3 ActionValue_X)
      (`self.AddMovementInput` _returnvalue_2 ActionValue_Y)
      (else
        (`self.AddMovementInput` _returnvalue_3 (/ ActionValue_X 2.0))
        (`self.AddMovementInput` _returnvalue_2 (/ ActionValue_Y 2.0)))))
  (:`Completed`
    (goto _label)))

(event `EnhancedInput|/Game/Blueprint/Input/IA_MouseCamera`
  (params (ActionValue :type "Vector2D Structure") (ElapsedSeconds :type "Float (double-precision)") (TriggeredSeconds :type "Float (double-precision)") (InputAction :type "InputAction Object Reference" :default "/Game/Blueprint/Input/IA_MouseCamera.IA_MouseCamera"))
  (:`Triggered`
    (`self.AddControllerYawInput` ActionValue_X)
    (`self.AddControllerPitchInput` (* ActionValue_Y -1.0))))

(event `EnhancedInput|/Game/Blueprint/Input/IA_Dash`
  (params (ActionValue :type Boolean) (ElapsedSeconds :type "Float (double-precision)") (TriggeredSeconds :type "Float (double-precision)") (InputAction :type "InputAction Object Reference" :default "/Game/Blueprint/Input/IA_Dash.IA_Dash"))
  (:`Triggered`
    (set `self.IsDash` ActionValue :!label _label_2))
  (:`Completed`
    (goto _label_2)))

(event `EnhancedInput|/Game/Blueprint/Input/IA_Interact`
  (params (ActionValue :type Boolean) (ElapsedSeconds :type "Float (double-precision)") (TriggeredSeconds :type "Float (double-precision)") (InputAction :type "InputAction Object Reference" :default "/Game/Blueprint/Input/IA_Interact.IA_Interact"))
  (:`Triggered`
    (bind _outhit (`KismetSystemLibrary.LineTraceSingle` (`SceneComponent.K2_GetComponentLocation` (`self.Camera`)) (`SceneComponent.K2_GetComponentLocation` (`self.Line_Direction`)) "TraceTypeQuery1"))
    (message `/Game/Blueprint/BPI_Interactable.Interact` (`.HitActor` (`GameplayStatics.BreakHitResult` _outhit)) self)))

(fn `UserConstructionScript`)