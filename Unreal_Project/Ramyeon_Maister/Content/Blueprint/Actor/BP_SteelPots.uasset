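; BP_SteelPots is an interactable stack of steel pots that exposes a display name.
; Its construction script spawns static meshes at fixed vertical intervals between MinHeightVector and MaxHeightVector, then adds a box component sized to the stack's height.
; Interacting unhides the SteelPot component on the passed BPMalty, leaving the stack itself unchanged.
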(event `/Game/Blueprint/BPI_Interactable.Interact`
  (params (BP_Malty :type "/Game/Blueprint/Actor/BP_Malty Object Reference"))
  (`SceneComponent.SetHiddenInGame` (`/Game/Blueprint/Actor/BP_Malty.Steel_Pot` BP_Malty) false false))

(fn `GetDisplayName`
  (returns (Display_Name :type Text))
  (return (`self.Object_Name`)))

(fn `UserConstructionScript`
  (bind (_maxheightvector_x _maxheightvector_y _maxheightvector_z) (`KismetMathLibrary.BreakVector` (`self.MaxHeightVector`)))
  (bind (_minheightvector_x _minheightvector_y _minheightvector_z) (`KismetMathLibrary.BreakVector` (`self.MinHeightVector`)))
  (bind _returnvalue (`KismetMathLibrary.FTrunc` (/ (- _maxheightvector_z _minheightvector_z) 5.0)))
  (for _index (range (+ _returnvalue 1))
    (`AddComponent|NODE_AddStaticMeshComponent-0` :`RelativeTransform` (`KismetMathLibrary.MakeTransform` (+ (`self.MinHeightVector`) (`KismetMathLibrary.MakeVector` 0.0 0.0 (* _index 5.0))) (`self.K2_GetActorRotation`))))
  (bind _returnvalue_2 (`AddComponent|NODE_AddBoxComponent-0` :`RelativeTransform` (`KismetMathLibrary.MakeTransform` (+ (`KismetMathLibrary.GetVectorArrayAverage` (`|MakeArray` (`self.MinHeightVector`) (`self.MaxHeightVector`))) (0.0 8.0 -3.0)))))
  (`BoxComponent.SetBoxExtent` _returnvalue_2 (`KismetMathLibrary.MakeVector` 8.0 13.0 (* (+ _returnvalue 1) 2.5)) true))